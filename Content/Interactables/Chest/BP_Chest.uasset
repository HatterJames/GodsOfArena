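; BP_Chest is an interactable chest whose lid opens while the ItemInteraction input is held and closes again on release.
; A box overlap enables player input and shows the UI_OpenChest prompt widget created on BeginPlay, and leaving the box reverses both.
; The LidOpening timeline drives the lid's pitch, playing on press and reversing on release.
; SetHighlight toggles custom depth rendering on the base and lid for highlighting.
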(event OnComponentBeginOverlap(Box)
  (params (OverlappedComponent :type Primitive%20Component%20Object%20Reference) (OtherActor :type Actor%20Object%20Reference) (OtherComp :type Primitive%20Component%20Object%20Reference) (OtherBodyIndex :type Integer) (bFromSweep :type Boolean) (SweepResult :type Hit%20Result%20Structure%20%28by%20ref%29))
  (Input|EnableInput (Game|GetPlayerController 0))
  (UserInterface|Viewport|AddtoViewport (Variables|Default|GetChestHUD) 0))

(event OnComponentEndOverlap(Box)
  (params (OverlappedComponent :type Primitive%20Component%20Object%20Reference) (OtherActor :type Actor%20Object%20Reference) (OtherComp :type Primitive%20Component%20Object%20Reference) (OtherBodyIndex :type Integer))
  (Input|DisableInput (Game|GetPlayerController 0))
  (Widget|RemovefromParent (Variables|Default|GetChestHUD)))

(event EventBeginPlay
  (bind _returnvalue (UserInterface|CreateWidget "/Game/Interactables/Chest/UI_OpenChest.UI_OpenChest_C"))
  (Variables|Default|SetChestHUD _returnvalue))

(event Input|ActionEvents|InputActionItemInteraction
  (params (Key :type Key%20Structure))
  (:Pressed
    (bind _lidfloat (Timeline|LidOpening Play)
      (:Update
        (Transformation|SetRelativeRotation (Variables|Default|GetLid) (Math|Rotator|MakeRotator 0.0 _lidfloat 0.0) false false))))
  (:Released
    (Timeline|LidOpening Reverse)))

(fn ConstructionScript)

(fn SetHighlight
  (params (Highlight? :type Boolean))
  (Rendering|SetRenderCustomDepth (Variables|Default|GetBase) Highlight?))