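; Interactable chest that opens its lid while an actor overlaps its interaction area and closes it when the overlap ends.
; A timeline drives the lid's pitch, playing on begin overlap and reversing on end.
; Overlap also shows or removes the UI_OpenChest widget created at BeginPlay and toggles custom-depth highlighting on base and lid.
; Begin overlap enables input on the overlapping actor, while end overlap disables the chest's own.
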(event OnComponentBeginOverlap(InteractableArea)
  (params (OverlappedComponent :type Primitive%20Component%20Object%20Reference) (OtherActor :type Actor%20Object%20Reference) (OtherComp :type Primitive%20Component%20Object%20Reference) (OtherBodyIndex :type Integer) (bFromSweep :type Boolean) (SweepResult :type Hit%20Result%20Structure%20%28by%20ref%29))
  (Input|EnableInput OtherActor (Game|GetPlayerController 0))
  (UserInterface|Viewport|AddtoViewport (Variables|Default|GetChestHud) 0)
  (CallFunction|SetHighlight true)
  (bind _openingoflid (Timeline|LidOpnening Play)
    (:Update
      (Transformation|SetRelativeRotation (Variables|Default|GetLid) (Math|Rotator|MakeRotator 0.0 _openingoflid 0.0) false false))))

(event OnComponentEndOverlap(InteractableArea)
  (params (OverlappedComponent :type Primitive%20Component%20Object%20Reference) (OtherActor :type Actor%20Object%20Reference) (OtherComp :type Primitive%20Component%20Object%20Reference) (OtherBodyIndex :type Integer))
  (Input|DisableInput (Game|GetPlayerController 0))
  (Widget|RemovefromParent (Variables|Default|GetChestHud))
  (CallFunction|SetHighlight false)
  (bind _openingoflid (Timeline|LidOpnening Reverse)
    (:Update
      (Transformation|SetRelativeRotation (Variables|Default|GetLid) (Math|Rotator|MakeRotator 0.0 _openingoflid 0.0) false false))))

(event EventBeginPlay
  (bind _returnvalue (UserInterface|CreateWidget "/Game/Interactables/Chest/UI_OpenChest.UI_OpenChest_C"))
  (Variables|Default|SetChestHud _returnvalue))

(fn ConstructionScript)

(fn SetHighlight
  (params (Highlight? :type Boolean))
  (Rendering|SetRenderCustomDepth (Variables|Default|GetBase) Highlight?))