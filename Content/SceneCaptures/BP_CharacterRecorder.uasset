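; BP_CharacterRecorder is a character stand-in, apparently for scene capture, that displays equipped armor and weapons on its skeletal mesh.
; On BeginPlay it passes itself to Player_One, and its EquipItem and UnEquipItem events call AttachItem and UnAttachItem.
; AttachItem replaces the slot's actor with a collision-free spawn, snapped to a socket named by the item's info; back slots accept weapons or armor.
; UnAttachItem destroys the slot's actor.
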(event EventBeginPlay
  (bind _asplayer_one (Utilities|Casting|CastToPlayer_One (Game|GetPlayerCharacter 0)))
  (Class|BPIRecorderComm|PassReference(Message) _asplayer_one self))

(event EventEquipItem
  (params (ItemInfo :type F%20Item%20Info%20Structure))
  (CallFunction|AttachItem ItemInfo))

(event EventUnEquipItem
  (params (ItemInfo :type F%20Item%20Info%20Structure))
  (CallFunction|UnAttachItem ItemInfo))

(fn ConstructionScript)

(fn AttachItem
  (params (ItemInfo :type F%20Item%20Info%20Structure))
  (bind (_itemclass _itemslot) (Utilities|Struct|BreakF_ItemInfo ItemInfo))
  (switch Utilities|FlowControl|Switch|SwitchonESlotType _itemslot
    (:NewEnumerator1
      (Utilities|IsValid (Variables|Default|GetHeadItem)
        (:Is%20Valid
          (Actor|DestroyActor (Variables|Default|GetHeadItem)))
        (:Is%20Not%20Valid
          _))
      (bind _returnvalue (Game|SpawnActorfromClass _itemclass (Transformation|GetActorTransform) "AlwaysSpawn" 0 0))
      (bind _output_get (Variables|Default|SetHeadItem _returnvalue))
      (bind _asbp_base_armor (Utilities|Casting|CastToBP_BaseArmor _output_get))
      (Transformation|AttachComponentToComponent _asbp_base_armor (Variables|Default|GetSkeletalMesh) (Utilities|Struct|BreakFArmorInfo (Variables|/Game/Interactables/Armor/BP_BaseArmor.BP_BaseArmor_C|GetArmorInfo _asbp_base_armor)) "SnapToTarget" "SnapToTarget" "SnapToTarget" true)
      (Collision|SetActorEnableCollision _asbp_base_armor false))
    (:NewEnumerator2
      (Utilities|IsValid (Variables|Default|GetTorsoItem)
        (:Is%20Valid
          (Actor|DestroyActor (Variables|Default|GetTorsoItem)))
        (:Is%20Not%20Valid
          _))
      (bind _returnvalue_2 (Game|SpawnActorfromClass _itemclass (Transformation|GetActorTransform) "AlwaysSpawn" 0 0))
      (bind _output_get_2 (Variables|Default|SetTorsoItem _returnvalue_2))
      (bind _asbp_base_armor_2 (Utilities|Casting|CastToBP_BaseArmor _output_get_2))
      (Transformation|AttachComponentToComponent _asbp_base_armor_2 (Variables|Default|GetSkeletalMesh) (Utilities|Struct|BreakFArmorInfo (Variables|/Game/Interactables/Armor/BP_BaseArmor.BP_BaseArmor_C|GetArmorInfo _asbp_base_armor_2)) "SnapToTarget" "SnapToTarget" "SnapToTarget" true)
      (Collision|SetActorEnableCollision _asbp_base_armor_2 false))
    (:NewEnumerator3
      (Utilities|IsValid (Variables|Default|GetLeftShoulderItem)
        (:Is%20Valid
          (Actor|DestroyActor (Variables|Default|GetLeftShoulderItem)))
        (:Is%20Not%20Valid
          _))
      (bind _returnvalue_3 (Game|SpawnActorfromClass _itemclass (Transformation|GetActorTransform) "AlwaysSpawn" 0 0))
      (bind _output_get_3 (Variables|Default|SetLeftShoulderItem _returnvalue_3))
      (bind _asbp_base_armor_3 (Utilities|Casting|CastToBP_BaseArmor _output_get_3))
      (Transformation|AttachComponentToComponent _asbp_base_armor_3 (Variables|Default|GetSkeletalMesh) (Utilities|Struct|BreakFArmorInfo (Variables|/Game/Interactables/Armor/BP_BaseArmor.BP_BaseArmor_C|GetArmorInfo _asbp_base_armor_3)) "SnapToTarget" "SnapToTarget" "SnapToTarget" true)
      (Collision|SetActorEnableCollision _asbp_base_armor_3 false))
    (:NewEnumerator4
      (Utilities|IsValid (Variables|Default|GetRightShoulderItem)
        (:Is%20Valid
          (Actor|DestroyActor (Variables|Default|GetRightShoulderItem)))
        (:Is%20Not%20Valid
          _))
      (bind _returnvalue_4 (Game|SpawnActorfromClass _itemclass (Transformation|GetActorTransform) "AlwaysSpawn" 0 0))
      (bind _output_get_4 (Variables|Default|SetRightShoulderItem _returnvalue_4))
      (bind _asbp_base_armor_4 (Utilities|Casting|CastToBP_BaseArmor _output_get_4))
      (Transformation|AttachComponentToComponent _asbp_base_armor_4 (Variables|Default|GetSkeletalMesh) (Utilities|Struct|BreakFArmorInfo (Variables|/Game/Interactables/Armor/BP_BaseArmor.BP_BaseArmor_C|GetArmorInfo _asbp_base_armor_4)) "SnapToTarget" "SnapToTarget" "SnapToTarget" true)
      (Collision|SetActorEnableCollision _asbp_base_armor_4 false))
    (:NewEnumerator5
      (Utilities|IsValid (Variables|Default|GetLeftForeArmItem)
        (:Is%20Valid
          (Actor|DestroyActor (Variables|Default|GetLeftForeArmItem)))
        (:Is%20Not%20Valid
          _))
      (bind _returnvalue_5 (Game|SpawnActorfromClass _itemclass (Transformation|GetActorTransform) "AlwaysSpawn" 0 0))
      (bind _output_get_5 (Variables|Default|SetLeftForeArmItem _returnvalue_5))
      (bind _asbp_base_armor_5 (Utilities|Casting|CastToBP_BaseArmor _output_get_5))
      (Transformation|AttachComponentToComponent _asbp_base_armor_5 (Variables|Default|GetSkeletalMesh) (Utilities|Struct|BreakFArmorInfo (Variables|/Game/Interactables/Armor/BP_BaseArmor.BP_BaseArmor_C|GetArmorInfo _asbp_base_armor_5)) "SnapToTarget" "SnapToTarget" "SnapToTarget" true)
      (Collision|SetActorEnableCollision _asbp_base_armor_5 false))
    (:NewEnumerator6
      (Utilities|IsValid (Variables|Default|GetRightForeArmItem)
        (:Is%20Valid
          (Actor|DestroyActor (Variables|Default|GetRightForeArmItem)))
        (:Is%20Not%20Valid
          _))
      (bind _returnvalue_6 (Game|SpawnActorfromClass _itemclass (Transformation|GetActorTransform) "AlwaysSpawn" 0 0))
      (bind _output_get_6 (Variables|Default|SetRightForeArmItem _returnvalue_6))
      (bind _asbp_base_armor_6 (Utilities|Casting|CastToBP_BaseArmor _output_get_6))
      (Transformation|AttachComponentToComponent _asbp_base_armor_6 (Variables|Default|GetSkeletalMesh) (Utilities|Struct|BreakFArmorInfo (Variables|/Game/Interactables/Armor/BP_BaseArmor.BP_BaseArmor_C|GetArmorInfo _asbp_base_armor_6)) "SnapToTarget" "SnapToTarget" "SnapToTarget" true)
      (Collision|SetActorEnableCollision _asbp_base_armor_6 false))
    (:NewEnumerator7
      (Utilities|IsValid (Variables|Default|GetWaistItem)
        (:Is%20Valid
          (Actor|DestroyActor (Variables|Default|GetWaistItem)))
        (:Is%20Not%20Valid
          _))
      (bind _returnvalue_7 (Game|SpawnActorfromClass _itemclass (Transformation|GetActorTransform) "AlwaysSpawn" 0 0))
      (bind _output_get_7 (Variables|Default|SetWaistItem _returnvalue_7))
      (bind _asbp_base_armor_7 (Utilities|Casting|CastToBP_BaseArmor _output_get_7))
      (Transformation|AttachComponentToComponent _asbp_base_armor_7 (Variables|Default|GetSkeletalMesh) (Utilities|Struct|BreakFArmorInfo (Variables|/Game/Interactables/Armor/BP_BaseArmor.BP_BaseArmor_C|GetArmorInfo _asbp_base_armor_7)) "SnapToTarget" "SnapToTarget" "SnapToTarget" true)
      (Collision|SetActorEnableCollision _asbp_base_armor_7 false))
    (:NewEnumerator8
      (Utilities|IsValid (Variables|Default|GetLeftLegItem)
        (:Is%20Valid
          (Actor|DestroyActor (Variables|Default|GetLeftLegItem)))
        (:Is%20Not%20Valid
          _))
      (bind _returnvalue_8 (Game|SpawnActorfromClass _itemclass (Transformation|GetActorTransform) "AlwaysSpawn" 0 0))
      (bind _output_get_8 (Variables|Default|SetLeftLegItem _returnvalue_8))
      (bind _asbp_base_armor_8 (Utilities|Casting|CastToBP_BaseArmor _output_get_8))
      (Transformation|AttachComponentToComponent _asbp_base_armor_8 (Variables|Default|GetSkeletalMesh) (Utilities|Struct|BreakFArmorInfo (Variables|/Game/Interactables/Armor/BP_BaseArmor.BP_BaseArmor_C|GetArmorInfo _asbp_base_armor_8)) "SnapToTarget" "SnapToTarget" "SnapToTarget" true)
      (Collision|SetActorEnableCollision _asbp_base_armor_8 false))
    (:NewEnumerator9
      (Utilities|IsValid (Variables|Default|GetRightLegItem)
        (:Is%20Valid
          (Actor|DestroyActor (Variables|Default|GetRightLegItem)))
        (:Is%20Not%20Valid
          _))
      (bind _returnvalue_9 (Game|SpawnActorfromClass _itemclass (Transformation|GetActorTransform) "AlwaysSpawn" 0 0))
      (bind _output_get_9 (Variables|Default|SetRightLegItem _returnvalue_9))
      (bind _asbp_base_armor_9 (Utilities|Casting|CastToBP_BaseArmor _output_get_9))
      (Transformation|AttachComponentToComponent _asbp_base_armor_9 (Variables|Default|GetSkeletalMesh) (Utilities|Struct|BreakFArmorInfo (Variables|/Game/Interactables/Armor/BP_BaseArmor.BP_BaseArmor_C|GetArmorInfo _asbp_base_armor_9)) "SnapToTarget" "SnapToTarget" "SnapToTarget" true)
      (Collision|SetActorEnableCollision _asbp_base_armor_9 false))
    (:NewEnumerator12
      (Utilities|IsValid (Variables|Default|GetRightWaistItem)
        (:Is%20Valid
          (Actor|DestroyActor (Variables|Default|GetRightWaistItem)))
        (:Is%20Not%20Valid
          _))
      (bind _returnvalue_10 (Game|SpawnActorfromClass _itemclass (Transformation|GetActorTransform) "AlwaysSpawn" 0 0))
      (bind _output_get_10 (Variables|Default|SetRightWaistItem _returnvalue_10))
      (bind _asbp_base_weapon (Utilities|Casting|CastToBP_BaseWeapon _output_get_10))
      (Transformation|AttachComponentToComponent _asbp_base_weapon (Variables|Default|GetSkeletalMesh) (Utilities|Struct|BreakFWeaponInfo (Variables|/Game/Interactables/Weapons/BP_BaseWeapon.BP_BaseWeapon_C|GetWeaponInfo _asbp_base_weapon)) "SnapToTarget" "SnapToTarget" "SnapToTarget" true)
      (Collision|SetActorEnableCollision _asbp_base_weapon false))
    (:NewEnumerator13
      (Utilities|IsValid (Variables|Default|GetLeftWaistItem)
        (:Is%20Valid
          (Actor|DestroyActor (Variables|Default|GetLeftWaistItem)))
        (:Is%20Not%20Valid
          _))
      (bind _returnvalue_11 (Game|SpawnActorfromClass _itemclass (Transformation|GetActorTransform) "AlwaysSpawn" 0 0))
      (bind _output_get_11 (Variables|Default|SetLeftWaistItem _returnvalue_11))
      (bind _asbp_base_weapon_2 (Utilities|Casting|CastToBP_BaseWeapon _output_get_11))
      (Transformation|AttachComponentToComponent _asbp_base_weapon_2 (Variables|Default|GetSkeletalMesh) (Utilities|Struct|BreakFWeaponInfo (Variables|/Game/Interactables/Weapons/BP_BaseWeapon.BP_BaseWeapon_C|GetWeaponInfo _asbp_base_weapon_2)) "SnapToTarget" "SnapToTarget" "SnapToTarget" true)
      (Collision|SetActorEnableCollision _asbp_base_weapon_2 false))
    (:NewEnumerator15
      (Utilities|IsValid (Variables|Default|GetBackRightItem)
        (:Is%20Valid
          (Actor|DestroyActor (Variables|Default|GetBackRightItem)))
        (:Is%20Not%20Valid
          _))
      (bind _returnvalue_12 (Game|SpawnActorfromClass _itemclass (Transformation|GetActorTransform) "AlwaysSpawn" 0 0))
      (bind _output_get_12 (Variables|Default|SetBackRightItem _returnvalue_12))
      (bind _asbp_base_weapon_3 (Utilities|Casting|CastToBP_BaseWeapon _output_get_12)
        (:then
          (Transformation|AttachComponentToComponent _asbp_base_weapon_3 (Variables|Default|GetSkeletalMesh) (Utilities|Struct|BreakFWeaponInfo (Variables|/Game/Interactables/Weapons/BP_BaseWeapon.BP_BaseWeapon_C|GetWeaponInfo _asbp_base_weapon_3)) "SnapToTarget" "SnapToTarget" "SnapToTarget" true)
          (Collision|SetActorEnableCollision _asbp_base_weapon_3 false))
        (:CastFailed
          (bind _asbp_base_armor_10 (Utilities|Casting|CastToBP_BaseArmor _output_get_12))
          (Transformation|AttachComponentToComponent _asbp_base_armor_10 (Variables|Default|GetSkeletalMesh) (Utilities|Struct|BreakFArmorInfo (Variables|/Game/Interactables/Armor/BP_BaseArmor.BP_BaseArmor_C|GetArmorInfo _asbp_base_armor_10)) "SnapToTarget" "SnapToTarget" "SnapToTarget" true)
          (Collision|SetActorEnableCollision _asbp_base_armor_10 false))))
    (:NewEnumerator16
      (Utilities|IsValid (Variables|Default|GetBackLeftItem)
        (:Is%20Valid
          (Actor|DestroyActor (Variables|Default|GetBackLeftItem)))
        (:Is%20Not%20Valid
          _))
      (bind _returnvalue_13 (Game|SpawnActorfromClass _itemclass (Transformation|GetActorTransform) "AlwaysSpawn" 0 0))
      (bind _output_get_13 (Variables|Default|SetBackLeftItem _returnvalue_13))
      (bind _asbp_base_weapon_4 (Utilities|Casting|CastToBP_BaseWeapon _output_get_13)
        (:then
          (Transformation|AttachComponentToComponent _asbp_base_weapon_4 (Variables|Default|GetSkeletalMesh) (Utilities|Struct|BreakFWeaponInfo (Variables|/Game/Interactables/Weapons/BP_BaseWeapon.BP_BaseWeapon_C|GetWeaponInfo _asbp_base_weapon_4)) "SnapToTarget" "SnapToTarget" "SnapToTarget" true)
          (Collision|SetActorEnableCollision _asbp_base_weapon_4 false))
        (:CastFailed
          (bind _asbp_base_armor_11 (Utilities|Casting|CastToBP_BaseArmor _output_get_13))
          (Transformation|AttachComponentToComponent _asbp_base_armor_11 (Variables|Default|GetSkeletalMesh) (Utilities|Struct|BreakFArmorInfo (Variables|/Game/Interactables/Armor/BP_BaseArmor.BP_BaseArmor_C|GetArmorInfo _asbp_base_armor_11)) "SnapToTarget" "SnapToTarget" "SnapToTarget" true)
          (Collision|SetActorEnableCollision _asbp_base_armor_11 false))))
    (:NewEnumerator18
      (Utilities|IsValid (Variables|Default|GetQuiverItem)
        (:Is%20Valid
          (Actor|DestroyActor (Variables|Default|GetQuiverItem)))
        (:Is%20Not%20Valid
          _))
      (bind _returnvalue_14 (Game|SpawnActorfromClass _itemclass (Transformation|GetActorTransform) "AlwaysSpawn" 0 0))
      (bind _output_get_14 (Variables|Default|SetQuiverItem _returnvalue_14))
      (bind _asbp_base_weapon_5 (Utilities|Casting|CastToBP_BaseWeapon _output_get_14))
      (Transformation|AttachComponentToComponent _asbp_base_weapon_5 (Variables|Default|GetSkeletalMesh) (Utilities|Struct|BreakFWeaponInfo (Variables|/Game/Interactables/Weapons/BP_BaseWeapon.BP_BaseWeapon_C|GetWeaponInfo _asbp_base_weapon_5)) "SnapToTarget" "SnapToTarget" "SnapToTarget" true)
      (Collision|SetActorEnableCollision _asbp_base_weapon_5 false))))

(fn UnAttachItem
  (params (ItemInfo :type F%20Item%20Info%20Structure))
  (switch Utilities|FlowControl|Switch|SwitchonESlotType (Utilities|Struct|BreakF_ItemInfo ItemInfo)
    (:NewEnumerator1
      (Actor|DestroyActor (Variables|Default|GetHeadItem)))
    (:NewEnumerator2
      (Actor|DestroyActor (Variables|Default|GetTorsoItem)))
    (:NewEnumerator3
      (Actor|DestroyActor (Variables|Default|GetLeftShoulderItem)))
    (:NewEnumerator4
      (Actor|DestroyActor (Variables|Default|GetRightShoulderItem)))
    (:NewEnumerator5
      (Actor|DestroyActor (Variables|Default|GetLeftForeArmItem)))
    (:NewEnumerator6
      (Actor|DestroyActor (Variables|Default|GetRightForeArmItem)))
    (:NewEnumerator7
      (Actor|DestroyActor (Variables|Default|GetWaistItem)))
    (:NewEnumerator8
      (Actor|DestroyActor (Variables|Default|GetLeftLegItem)))
    (:NewEnumerator9
      (Actor|DestroyActor (Variables|Default|GetRightLegItem)))
    (:NewEnumerator12
      (Actor|DestroyActor (Variables|Default|GetRightWaistItem)))
    (:NewEnumerator13
      (Actor|DestroyActor (Variables|Default|GetLeftWaistItem)))
    (:NewEnumerator15
      (Actor|DestroyActor (Variables|Default|GetBackRightItem)))
    (:NewEnumerator16
      (Actor|DestroyActor (Variables|Default|GetBackLeftItem)))
    (:NewEnumerator18
      (Actor|DestroyActor (Variables|Default|GetQuiverItem)))))